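; BP_HyperMove_IP is an interaction point for hyper moves, shown as three spinning rings at staggered angles.
; Interact, burst and pass zones report overlaps to the overlapping actor through zone messages, with interact and burst radii set at construction.
; When triggered, it sends its move type and action data to the caller once until ResetTrigger clears the latch.
; PassedZone fires a passed-point dispatcher.
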(event `self.ReceiveTick`
  (params (DeltaSeconds :type "Float (single-precision)"))
  (bind _output_get (set `self.AnimAngle` (+ (stale _output_get) (* DeltaSeconds 360.0))))
  (`SceneComponent.K2_SetRelativeRotation` (`self.ring1`) (`KismetMathLibrary.RotatorFromAxisAndAngle` (1.0 -1.0 1.0) _output_get) false false)
  (`SceneComponent.K2_SetRelativeRotation` (`self.ring2`) (`KismetMathLibrary.RotatorFromAxisAndAngle` (1.0 1.0 1.0) (- _output_get 120.0)) false false)
  (`SceneComponent.K2_SetRelativeRotation` (`self.ring3`) (`KismetMathLibrary.RotatorFromAxisAndAngle` (1.0 1.0 -1.0) (- _output_get 240.0)) false false))

(event `self.InteractZone.OnComponentBeginOverlap`
  (params (OverlappedComponent :type "PrimitiveComponent Object Reference") (OtherActor :type "Actor Object Reference") (OtherComp :type "PrimitiveComponent Object Reference") (OtherBodyIndex :type Integer) (bFromSweep :type Boolean) (SweepResult :type "HitResult Structure (by ref)"))
  (message `/Game/BPs/Interfaces/BI_HyperMove.EnteredZone` OtherActor "NewEnumerator0" self))

(event `self.InteractZone.OnComponentEndOverlap`
  (params (OverlappedComponent :type "PrimitiveComponent Object Reference") (OtherActor :type "Actor Object Reference") (OtherComp :type "PrimitiveComponent Object Reference") (OtherBodyIndex :type Integer))
  (message `/Game/BPs/Interfaces/BI_HyperMove.LeftZone` OtherActor "NewEnumerator0" self))

(event `self.PassZone.OnComponentBeginOverlap`
  (params (OverlappedComponent :type "PrimitiveComponent Object Reference") (OtherActor :type "Actor Object Reference") (OtherComp :type "PrimitiveComponent Object Reference") (OtherBodyIndex :type Integer) (bFromSweep :type Boolean) (SweepResult :type "HitResult Structure (by ref)"))
  (message `/Game/BPs/Interfaces/BI_HyperMove.EnteredZone` OtherActor "NewEnumerator4" self))

(event `/Game/BPs/Interfaces/BI_HyperMove.PassedZone`
  (`self.PassedPointEventDispatcher`))

(event `/Game/BPs/Interfaces/BI_HyperMove.TriggerHyperMoveInteractionAction`
  (params (HyperMoveType :type "/Game/BPs/Data/Enums/E_HyperMoveInteractType Enum" :default "NewEnumerator3") (metadata :type "/Game/BPs/Data/Structs/F_HyperMoveInteractionActionData Structure") (Caller :type "Actor Object Reference"))
  (if (not (`self.bTriggered`))
    (message `/Game/BPs/Interfaces/BI_HyperMove.TriggerHyperMoveInteractionAction` Caller (`self.HyperMoveIneractType`) (`self.InteractionActionData`) null)
    (set `self.bTriggered` true)))

(event `self.BurstZone.OnComponentBeginOverlap`
  (params (OverlappedComponent :type "PrimitiveComponent Object Reference") (OtherActor :type "Actor Object Reference") (OtherComp :type "PrimitiveComponent Object Reference") (OtherBodyIndex :type Integer) (bFromSweep :type Boolean) (SweepResult :type "HitResult Structure (by ref)"))
  (message `/Game/BPs/Interfaces/BI_HyperMove.EnteredZone` OtherActor "NewEnumerator1" self))

(event `self.BurstZone.OnComponentEndOverlap`
  (params (OverlappedComponent :type "PrimitiveComponent Object Reference") (OtherActor :type "Actor Object Reference") (OtherComp :type "PrimitiveComponent Object Reference") (OtherBodyIndex :type Integer))
  (message `/Game/BPs/Interfaces/BI_HyperMove.LeftZone` OtherActor "NewEnumerator1" self))

(fn `ResetTrigger`
  (set `self.bTriggered` false)
  (return))

(fn `UserConstructionScript`
  (bind _dirin (`self.DirIn`))
  (`SphereComponent.SetSphereRadius` (`self.BurstZone`) (`self.BurstZoneRadius`) true)
  (`SphereComponent.SetSphereRadius` (`self.InteractZone`) (`self.InteractZoneRadius`) true)
  (`SceneComponent.K2_SetRelativeLocation` (`self.DirIn`) (`KismetMathLibrary.MakeVector` (* (`ArrowComponent.ArrowLength` _dirin) -1.0 (`ArrowComponent.ArrowSize` _dirin))) false false))