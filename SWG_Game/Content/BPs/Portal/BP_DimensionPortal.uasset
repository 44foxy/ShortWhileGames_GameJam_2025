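; BP_DimensionPortal is a portal that breaks when the player completes a run through its linked points.
; It counts pass events from LinkedIPs during an engaged run; overlapping the portal with all passed sends a zone message and calls the portal-broke dispatcher.
; The Entry volume, placed at EntryPointLocation on construction, reports enter and leave to the overlapping actor.
; Engaging or disengaging a run resets the counter; disengaging also resets point triggers.
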(event `self.ReceiveBeginPlay`
  (bind _linkedips (`self.LinkedIPs`))
  (for _array_element _linkedips
    (add `/Game/BPs/Interactible/BP_HyperMove_IP.PassedPointEventDispatcher` _array_element (`|CreateDelegate` :!event `PlayerPassedPoint`)))
  (`KismetSystemLibrary.PrintText` (`|FormatText` "Linked IPs count: {c}" (`KismetArrayLibrary.Array_Length` _linkedips)) true true (struct :`G` 0.66 :`B` 1.0 :`A` 1.0) 2.0 "DPO_init"))

(event `PlayerPassedPoint`
  (if (`self.PlayerEngagedInRun`)
    (`/Engine/EditorBlueprintResources/StandardMacros.IncrementInt` (`self.PassedIPsCounter`)
      (:`  `
        (`KismetSystemLibrary.PrintText` "Player passed point" true true (struct :`R` 1.0 :`B` 0.049266 :`A` 1.0) 2.0 "None")))))

(event `self.Portal.OnComponentBeginOverlap`
  (params (OverlappedComponent :type "PrimitiveComponent Object Reference") (OtherActor :type "Actor Object Reference") (OtherComp :type "PrimitiveComponent Object Reference") (OtherBodyIndex :type Integer) (bFromSweep :type Boolean) (SweepResult :type "HitResult Structure (by ref)"))
  (if (and (`self.PlayerEngagedInRun`) (== (`self.PassedIPsCounter`) (`KismetArrayLibrary.Array_Length` (`self.LinkedIPs`))))
    (message `/Game/BPs/Interfaces/BI_HyperMove.EnteredZone` OtherActor "NewEnumerator3" self)
    (`self.PortalBrokeEventSipatcher`)
    (`KismetSystemLibrary.PrintText` "Player trigered portal break" true true (struct :`R` 1.0 :`B` 0.049266 :`A` 1.0) 2.0 "None")))

(event `self.Entry.OnComponentBeginOverlap`
  (params (OverlappedComponent :type "PrimitiveComponent Object Reference") (OtherActor :type "Actor Object Reference") (OtherComp :type "PrimitiveComponent Object Reference") (OtherBodyIndex :type Integer) (bFromSweep :type Boolean) (SweepResult :type "HitResult Structure (by ref)"))
  (message `/Game/BPs/Interfaces/BI_HyperMove.EnteredZone` OtherActor "NewEnumerator2" self)
  (`KismetSystemLibrary.PrintText` "Player entered entry zone" true true (struct :`R` 1.0 :`B` 0.049266 :`A` 1.0) 2.0 "None"))

(event `self.Entry.OnComponentEndOverlap`
  (params (OverlappedComponent :type "PrimitiveComponent Object Reference") (OtherActor :type "Actor Object Reference") (OtherComp :type "PrimitiveComponent Object Reference") (OtherBodyIndex :type Integer))
  (message `/Game/BPs/Interfaces/BI_HyperMove.LeftZone` OtherActor "NewEnumerator2" self)
  (`KismetSystemLibrary.PrintText` "Player left entry zone" true true (struct :`R` 1.0 :`B` 0.049266 :`A` 1.0) 2.0 "None"))

(event `/Game/BPs/Interfaces/BI_HyperMove.PortalRunEngaged`
  (set `self.PlayerEngagedInRun` true)
  (set `self.PassedIPsCounter` 0 :!label _label)
  (`KismetSystemLibrary.PrintText` (`|FormatText` "Run engaged: {b}" (`self.PlayerEngagedInRun`)) true true (struct :`R` 1.0 :`B` 0.049266 :`A` 1.0) 2.0 "None"))

(event `/Game/BPs/Interfaces/BI_HyperMove.PortalRunDisengaged`
  (`|ExecutionSequence`
    (:`then_0`
      (set `self.PlayerEngagedInRun` false)
      (goto _label))
    (:`then_1`
      (for _array_element (`self.LinkedIPs`)
        (`/Game/BPs/Interactible/BP_HyperMove_IP.ResetTrigger` _array_element)))))

(fn `UserConstructionScript`
  (bind _entrypointlocation (`self.EntryPointLocation`))
  (`/Engine/EditorBlueprintResources/StandardMacros.IsValid` _entrypointlocation
    (:`Is Valid`
      (`SceneComponent.K2_SetWorldLocation` (`self.Entry`) (`SceneComponent.K2_GetComponentLocation` (`Actor.RootComponent` _entrypointlocation)) false false))))