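; BP_InteractFoliage merges placed FoliageInstance actors of one Type into a single instanced static mesh.
; The construction script picks a cube or sphere mesh from the Type setting.
; On BeginPlay it adds a world-space instance at the root transform of each FoliageInstance with matching Type.
; It then destroys every FoliageInstance in the level, including those of other types.
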(event `self.ReceiveBeginPlay`
  (bind _outactors (`GameplayStatics.GetAllActorsOfClass` "/Game/Core/FoliageInstance.FoliageInstance_C"))
  (for _array_element _outactors
    (if (`|EnumEquality` (`/Game/Core/FoliageInstance.Type` _array_element) (`self.Type`))
      (`InstancedStaticMeshComponent.AddInstance` (`self.InstancedStaticMesh`) (`SceneComponent.K2_GetComponentToWorld` (`/Game/Core/FoliageInstance.DefaultSceneRoot` _array_element)) true)))
  (for _array_element_2 _outactors
    (`self.K2_DestroyActor` _array_element_2)))

(fn `UserConstructionScript`
  (`StaticMeshComponent.SetStaticMesh` (`self.InstancedStaticMesh`) (select `/Game/Core/FoliageType` (`self.Type`) :`NewEnumerator0` "/Engine/BasicShapes/Cube.Cube" :`NewEnumerator1` "/Engine/EditorMeshes/EditorSphere.EditorSphere" :!type "StaticMesh Object Reference")))