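; BP_Player is a player Blueprint that serves as a test harness for writing HP on a UI widget.
; BeginPlay creates UW_tst and UW_tst254 and adds both to the viewport.
; Every Tick runs MyTest, which calls SetHP on UW_tst254, then NormalTest, which assigns its HP directly, each printing a keyed message.
; The T debug key only prints text, and the Blueprint's own SetHP is an empty stub.
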(event EventBeginPlay
  (bind _returnvalue (Game|GetPlayerController 0))
  (bind _returnvalue_2 (UserInterface|CreateWidget "/Game/Core/Player/HUD/UW_tst.UW_tst_C" _returnvalue))
  (bind _returnvalue_3 (UserInterface|CreateWidget "/Game/Core/Player/HUD/UW_tst254.UW_tst254_C" _returnvalue))
  (Utilities|FlowControl|Sequence
    (:then_0
      (Utilities|FlowControl|Sequence
        (:then_0
          (UserInterface|Viewport|AddtoViewport _returnvalue_2 0))
        (:then_1
          (UserInterface|Viewport|AddtoViewport _returnvalue_3 0))))))

(event Collision|EventActorBeginOverlap
  (params (OtherActor :type Actor%20Object%20Reference)))

(event EventTick
  (params (DeltaSeconds :type Float%20%28single-precision%29))
  (Utilities|FlowControl|Sequence
    (:then_0
      (CallFunction|MyTest (stale EventBeginPlay _returnvalue_3)))
    (:then_1
      (CallFunction|NormalTest (stale EventBeginPlay _returnvalue_3)))))

(event Input|KeyboardEvents|DebugKeyT
  (params (Key :type Key%20Structure) (ActionValue :type Input%20Action%20Value%20Structure))
  (:Pressed
    (Development|PrintString "add")))

(fn ConstructionScript)

(fn MyTest
  (params (self2 :type BI%20Player%20HUD%20Interface))
  (Default|SetHP self2 0.5)
  (Development|PrintString "MyDone" true true "(R=0.000000,G=0.660000,B=1.000000,A=1.000000)" 2.0 "MD"))

(fn NormalTest
  (params (self2 :type UW%20Tst%20254%20Object%20Reference))
  (Variables|/Game/Core/Player/HUD/UW_tst254.UW_tst254_C|SetHP self2 0.0)
  (Development|PrintString "NormalDone" true true "(R=0.000000,G=0.660000,B=1.000000,A=1.000000)" 2.0 "ND"))

(fn SetHP
  (params (NewHP :type Float%20%28double-precision%29))
  (return))