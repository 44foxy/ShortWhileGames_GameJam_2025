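; Player pawn with custom inertia-based movement that toggles between a standard mode and a fast, auto-accelerating hyper mode with yaw momentum.
; Each tick it decelerates axes, projects speed along ground directions from paired line traces, applies gravity when airborne, snaps to ground, and sweeps the actor.
; Swapping modes switches Enhanced Input contexts and carries speed over.
; Zone events gate portal runs, super-shift turns and triggered jumps; speed drives FOV, tilt and animation.
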(event `self.ReceiveBeginPlay`
  (`EnhancedInputSubsystemInterface.AddMappingContext` (pcsubsystem `EnhancedInputLocalPlayerSubsystem` (`GameplayStatics.GetPlayerController` 0)) "/Game/Core/Input/Standard/IMC_Standard.IMC_Standard" 0 (struct))
  (`GameplayStatics.SetGlobalTimeDilation` 1.0))

(event `Deceleration`
  (bind _dt (`self.DT`))
  (bind _bgrounded (`self.bGrounded`))
  ; Deceleration
  (if (`self.Debug`)
    _
    (elif (`.bHyperMode_10_63D6054647C30321204495B9C3DB90EB` (break `/Game/BPs/Data/Structs/F_HyperMoveData` (`self.HyperMoveData`)))
      (if _bgrounded
        (`self.DecelerateAxis` _dt (`self.SideAxis_S`)))
      (elif _bgrounded
        (`self.DecelerateAxis` _dt (`self.FrontAxis_S`))
        (`self.DecelerateAxis` _dt (`self.SideAxis_S`))
        (`self.DecelerateAxis` _dt (`self.FrontAxis_Hyper`))))))

(event `self.ReceiveTick`
  (params (DeltaSeconds :type "Float (single-precision)"))
  (set `self.DT` DeltaSeconds)
  (`|ExecutionSequence`
    (:`then_0`
      (if (`self.Debug`)
        (setmembers `/Game/BPs/Data/Structs/F_AxisInertia` :`StructRef` (`self.FrontAxis_S`) :`CurrentSpeed` 1000.0)))
    (:`then_1`
      (`|ExecutionSequence`
        (:`then_0`
          (`self.Deceleration`))
        (:`then_1`
          (`self.XYInertiaCompute`))
        (:`then_2`
          (`self.GroundVectorsAndInertiaCompute`))
        (:`then_3`
          (`self.ApplyInertia`))
        (:`then_4`
          (`self.HyperRotation`))
        (:`then_5`
          (`self.SpeedEffects`))
        (:`then_6`
          (`self.Animation`))))))

(event `XYInertiaCompute`
  (bind _dt (`self.DT`))
  ; XY local inertia vector combine
  (if (`self.Debug`)
    _
    (elif (not (`.bHyperMode_10_63D6054647C30321204495B9C3DB90EB` (break `/Game/BPs/Data/Structs/F_HyperMoveData` (`self.HyperMoveData`))))
      (set `self.XYBaseInertiaVector` (`KismetMathLibrary.GreaterGreater_VectorRotator` (`KismetMathLibrary.MakeVector` (* (`.CurrentSpeed_48_BCC8F5724ACD309D8CD3E488248F36B0` (break `/Game/BPs/Data/Structs/F_AxisInertia` (`self.FrontAxis_S`))) _dt) (* (`.CurrentSpeed_48_BCC8F5724ACD309D8CD3E488248F36B0` (break `/Game/BPs/Data/Structs/F_AxisInertia` (`self.SideAxis_S`))) _dt)) (`SceneComponent.K2_GetComponentRotation` (`self.Capsule`)))))))

(event `GroundVectorsAndInertiaCompute`
  (bind _bgrounded (`self.bGrounded`))
  ; Ground direction vector calculation
  (bind (_forwardhit _forwarddirection _sidehit _sidedirection) (`self.GetMultiGroundDirectionalVector`))
  (`|ExecutionSequence`
    (:`then_0`
      (if (and _forwardhit _bgrounded)
        (bind _output_get (set `self.LastKnownGroundDirection_forward` _forwarddirection))
        (else
          ;;[0 0.0313 0.3854 0.5] Apply integrated gravity if not grounded
          (set `self.ComposedInertia` (+ (`self.ComposedInertia`) (* (0.0 0.0 -980.0) (`self.DT`) 1.0))))))
    (:`then_1`
      (if (and _sidehit _bgrounded)
        (bind _output_get_2 (set `self.LastKnownGroundDirection_side` _sidedirection))))
    (:`then_2`
      (if _bgrounded
        (set `self.ComposedInertia` (+ (* _output_get (`KismetMathLibrary.SelectFloat` (`.CurrentSpeed_48_BCC8F5724ACD309D8CD3E488248F36B0` (break `/Game/BPs/Data/Structs/F_AxisInertia` (`self.FrontAxis_Hyper`))) (`.CurrentSpeed_48_BCC8F5724ACD309D8CD3E488248F36B0` (break `/Game/BPs/Data/Structs/F_AxisInertia` (`self.FrontAxis_S`))) (`.bHyperMode_10_63D6054647C30321204495B9C3DB90EB` (break `/Game/BPs/Data/Structs/F_HyperMoveData` (`self.HyperMoveData`))))) (* _output_get_2 (`.CurrentSpeed_48_BCC8F5724ACD309D8CD3E488248F36B0` (break `/Game/BPs/Data/Structs/F_AxisInertia` (`self.SideAxis_S`))))))))
    (:`then_3`
      (bind _returnvalue (`self.GroundCheckOffset`))
      (set `self.bGrounded` _returnvalue))))

(event `Animation`
  (bind (_axis _currentspeed _isbeingchanged _accel _decel _bypassdecel _maxpositive) (break `/Game/BPs/Data/Structs/F_AxisInertia` (`self.FrontAxis_S`)))
  (bind _bhypermode (break `/Game/BPs/Data/Structs/F_HyperMoveData` (`self.HyperMoveData`)))
  (bind (_axis_2 _currentspeed_2 _isbeingchanged_2 _accel_2 _decel_2 _bypassdecel_2 _maxpositive_2) (break `/Game/BPs/Data/Structs/F_AxisInertia` (`self.FrontAxis_Hyper`)))
  ; Animation
  (`|ExecutionSequence`
    (:`then_0`
      (message `/Game/Models/Player/BI_Anim.SetAnimState` (`SkeletalMeshComponent.GetAnimInstance` (`self.SKM_Player`)) (`KismetMathLibrary.SelectFloat` (`KismetMathLibrary.MapRangeClamped` _currentspeed_2 0.0 _maxpositive_2 0.0 100.0) (`KismetMathLibrary.MapRangeClamped` _currentspeed 0.0 _maxpositive 0.0 50.0) _bhypermode)))
    (:`then_1`
      (`SceneComponent.K2_SetRelativeRotation` (`self.RootRot`) (`KismetMathLibrary.MakeRotator` 0.0 (`KismetMathLibrary.SelectFloat` (`KismetMathLibrary.MapRangeClamped` _currentspeed_2 0.0 _maxpositive_2 0.0 -40.0) (`KismetMathLibrary.MapRangeClamped` _currentspeed 0.0 _maxpositive 0.0 -20.0) _bhypermode)) false false))))

(event `ApplyInertia`
  (bind _composedinertia (`self.ComposedInertia`))
  ; Move pawn and check for ground
  (`self.K2_AddActorWorldOffset` (* _composedinertia (`self.DT`) 1.0) true)
  (`KismetSystemLibrary.PrintString` (`KismetStringLibrary.Conv_VectorToString` _composedinertia) true true (struct :`G` 0.66 :`B` 1.0 :`A` 1.0) 10000.0 "cmpsd")
  (if (`.bHyperMode_10_63D6054647C30321204495B9C3DB90EB` (break `/Game/BPs/Data/Structs/F_HyperMoveData` (`self.HyperMoveData`)))
    (`self.AccelerateAxis` (`self.FrontAxis_Hyper`) 1.0)))

(event `HyperRotation`
  (bind (_bhypermode _evaluatingininteractzone _yawmomentum) (break `/Game/BPs/Data/Structs/F_HyperMoveData` (`self.HyperMoveData`)))
  (bind (_axis _currentspeed _isbeingchanged _accel _decel _bypassdecel _maxpositive) (break `/Game/BPs/Data/Structs/F_AxisInertia` (`self.FrontAxis_Hyper`)))
  ; HyperRotation
  (if (and (`self.bGrounded`) _bhypermode)
    (`SceneComponent.K2_AddLocalRotation` (`self.Capsule`) (`KismetMathLibrary.MakeRotator` 0.0 0.0 (* (* _yawmomentum (`self.DT`)) (/ _currentspeed _maxpositive))) false false)))

(event `SpeedEffects`
  (bind (_axis _currentspeed _isbeingchanged _accel _decel _bypassdecel _maxpositive) (break `/Game/BPs/Data/Structs/F_AxisInertia` (`self.FrontAxis_Hyper`)))
  (bind (_axis_2 _currentspeed_2 _isbeingchanged_2 _accel_2 _decel_2 _bypassdecel_2 _maxpositive_2) (break `/Game/BPs/Data/Structs/F_AxisInertia` (`self.FrontAxis_S`)))
  ; Speed effects
  (`CameraComponent.SetFieldOfView` (`self.Camera`) (`KismetMathLibrary.SelectFloat` (`KismetMathLibrary.MapRangeClamped` _currentspeed 0.0 _maxpositive 90.0 120.0) (`KismetMathLibrary.MapRangeUnclamped` _currentspeed_2 0.0 _maxpositive_2 90.0 105.0) (> _currentspeed _currentspeed_2))))

(event `EnhancedInput|/Game/Core/Input/Standard/IA_Move_Standard`
  (params (ActionValue :type "Vector2D Structure") (ElapsedSeconds :type "Float (double-precision)") (TriggeredSeconds :type "Float (double-precision)") (InputAction :type "InputAction Object Reference" :default "/Game/Core/Input/Standard/IA_Move_Standard.IA_Move_Standard"))
  (:`Triggered`
    (`|ExecutionSequence`
      (:`then_0`
        (`self.AccelerateAxis` (`self.FrontAxis_S`) ActionValue_X :!label _label))
      (:`then_1`
        (`self.AccelerateAxis` (`self.SideAxis_S`) ActionValue_Y :!label _label_2))))
  (:`Completed`
    (`|ExecutionSequence`
      (:`then_0`
        (goto _label))
      (:`then_1`
        (goto _label_2)))))

(event `EnhancedInput|/Game/Core/Input/Standard/IA_Rotate_Standard`
  (params (ActionValue :type "Float (double-precision)") (ElapsedSeconds :type "Float (double-precision)") (TriggeredSeconds :type "Float (double-precision)") (InputAction :type "InputAction Object Reference" :default "/Game/Core/Input/Standard/IA_Rotate_Standard.IA_Rotate_Standard"))
  (:`Triggered`
    (if (`self.bGrounded`)
      (`SceneComponent.K2_AddLocalRotation` (`self.Root`) (`KismetMathLibrary.MakeRotator` 0.0 0.0 (`KismetMathLibrary.FClamp` (* ActionValue (`GameplayStatics.GetWorldDeltaSeconds`) (`self.RotationSense`)) -10.0 10.0)) false false))))

(event `EnhancedInput|/Game/Core/Input/Hyper/IA_Rotate_Hyper`
  (params (ActionValue :type "Float (double-precision)") (ElapsedSeconds :type "Float (double-precision)") (TriggeredSeconds :type "Float (double-precision)") (InputAction :type "InputAction Object Reference" :default "/Game/Core/Input/Hyper/IA_Rotate_Hyper.IA_Rotate_Hyper"))
  (bind _hypermovedata (`self.HyperMoveData`))
  (bind (_bhypermode _evaluatingininteractzone _yawmomentum) (break `/Game/BPs/Data/Structs/F_HyperMoveData` _hypermovedata))
  (:`Triggered`
    (set `self.HyperRotSaveState` ActionValue)
    (if (`self.bInSuperShift`)
      (setmembers `/Game/BPs/Data/Structs/F_HyperMoveData` :`StructRef` _hypermovedata :`YawMomentum` 0.0)
      (else
        (setmembers `/Game/BPs/Data/Structs/F_HyperMoveData` :`StructRef` _hypermovedata :`YawMomentum` (`KismetMathLibrary.FClamp` (+ _yawmomentum (* ActionValue 0.4)) -60.0 60.0))
        (`KismetSystemLibrary.PrintString` (`KismetStringLibrary.Conv_DoubleToString` _yawmomentum) true true (struct :`G` 0.66 :`B` 1.0 :`A` 1.0) 2.0 "msx"))))
  (:`Completed`
    (set `self.HyperRotSaveState` 0.0)))

(event `EnhancedInput|/Game/Core/Input/Hyper/IA_HyperInteract`
  (params (ActionValue :type Boolean) (ElapsedSeconds :type "Float (double-precision)") (TriggeredSeconds :type "Float (double-precision)") (InputAction :type "InputAction Object Reference" :default "/Game/Core/Input/Hyper/IA_HyperInteract.IA_HyperInteract"))
  (bind _portalsystemdata (`self.PortalSystemData`))
  (:`Triggered`
    (if (`.ReadyAtEntry_8_8FBACF50406485D6BFB61A88F323A605` (break `/Game/BPs/Data/Structs/F_PortalSystemData` _portalsystemdata))
      (setmembers `/Game/BPs/Data/Structs/F_PortalSystemData` :`StructRef` _portalsystemdata :`ReadyAtEntry` false :`EngagedInRun` true)
      (`self.EngagePortalRun`))))

(event `EnhancedInput|/Game/Core/Input/Hyper/IA_SuperShift`
  (params (ActionValue :type Boolean) (ElapsedSeconds :type "Float (double-precision)") (TriggeredSeconds :type "Float (double-precision)") (InputAction :type "InputAction Object Reference" :default "/Game/Core/Input/Hyper/IA_SuperShift.IA_SuperShift"))
  (bind (_readyatentry _engagedinrun _dimensionportal _readyforinteracttrigger _currentzoneactor) (break `/Game/BPs/Data/Structs/F_PortalSystemData` (`self.PortalSystemData`)))
  (:`Started`
    (if (and _engagedinrun _readyforinteracttrigger)
      (message `/Game/BPs/Interfaces/BI_HyperMove.TriggerHyperMoveInteractionAction` _currentzoneactor "NewEnumerator3" (struct) self))))

(event `EnhancedInput|/Game/Core/Input/Hyper/IA_LeftSuperShift`
  (params (ActionValue :type Boolean) (ElapsedSeconds :type "Float (double-precision)") (TriggeredSeconds :type "Float (double-precision)") (InputAction :type "InputAction Object Reference" :default "/Game/Core/Input/Hyper/IA_LeftSuperShift.IA_LeftSuperShift"))
  (bind _hyperrotsavestate (`self.HyperRotSaveState`))
  (bind _returnvalue (* _hyperrotsavestate 20.0 (`self.DT`)))
  (:`Triggered`
    (if (and (< _hyperrotsavestate 0.0) (`.ReadyForSuperShift_15_99A194CA4D1719876D027D9A531E35BB` (break `/Game/BPs/Data/Structs/F_PortalSystemData` (`self.PortalSystemData`))) (xor ActionValue (stale `EnhancedInput|/Game/Core/Input/Hyper/IA_RightSuperShift` ActionValue)))
      (set `self.bInSuperShift` true)
      (`SceneComponent.K2_AddLocalRotation` (`self.Capsule`) (`KismetMathLibrary.MakeRotator` 0.0 0.0 _returnvalue) false false)
      (if (not (`self.bGrounded`))
        (set `self.ComposedInertia` (`KismetMathLibrary.RotateAngleAxis` (`self.ComposedInertia`) _returnvalue (0.0 0.0 1.0))))))
  (:`Completed`
    (set `self.bInSuperShift` false :!label _label)))

(event `EnhancedInput|/Game/Core/Input/Hyper/IA_RightSuperShift`
  (params (ActionValue :type Boolean) (ElapsedSeconds :type "Float (double-precision)") (TriggeredSeconds :type "Float (double-precision)") (InputAction :type "InputAction Object Reference" :default "/Game/Core/Input/Hyper/IA_RightSuperShift.IA_RightSuperShift"))
  (bind _hyperrotsavestate (`self.HyperRotSaveState`))
  (bind _returnvalue (* _hyperrotsavestate 20.0 (`self.DT`)))
  (:`Triggered`
    (if (and (`.ReadyForSuperShift_15_99A194CA4D1719876D027D9A531E35BB` (break `/Game/BPs/Data/Structs/F_PortalSystemData` (`self.PortalSystemData`))) (> _hyperrotsavestate 0.0) (xor (stale `EnhancedInput|/Game/Core/Input/Hyper/IA_LeftSuperShift` ActionValue) ActionValue))
      (set `self.bInSuperShift` true)
      (`SceneComponent.K2_AddLocalRotation` (`self.Capsule`) (`KismetMathLibrary.MakeRotator` 0.0 0.0 _returnvalue) false false)
      (if (not (`self.bGrounded`))
        (set `self.ComposedInertia` (`KismetMathLibrary.RotateAngleAxis` (`self.ComposedInertia`) _returnvalue (0.0 0.0 1.0))))))
  (:`Completed`
    (goto _label)))

(event `EnhancedInput|/Game/Core/Input/IA_ModeToggle`
  (params (ActionValue :type Boolean) (ElapsedSeconds :type "Float (double-precision)") (TriggeredSeconds :type "Float (double-precision)") (InputAction :type "InputAction Object Reference" :default "/Game/Core/Input/IA_ModeToggle.IA_ModeToggle"))
  (:`Started`
    (`self.SwapMovementMode` (not (`.bHyperMode_10_63D6054647C30321204495B9C3DB90EB` (break `/Game/BPs/Data/Structs/F_HyperMoveData` (`self.HyperMoveData`)))))))

(event `/Game/BPs/Interfaces/BI_HyperMove.EnteredZone`
  (params (ZoneType :type "/Game/BPs/Data/Enums/E_HyperZoneType Enum" :default "NewEnumerator0") (ZoneActorRef :type "Actor Object Reference"))
  (bind _portalsystemdata (`self.PortalSystemData`))
  (bind (_readyatentry _engagedinrun _dimensionportal) (break `/Game/BPs/Data/Structs/F_PortalSystemData` _portalsystemdata))
  (switch `/Game/BPs/Data/Enums/E_HyperZoneType` ZoneType
    (:`NewEnumerator0`
      (if _engagedinrun
        (setmembers `/Game/BPs/Data/Structs/F_PortalSystemData` :`StructRef` _portalsystemdata :`ReadyForSuperShift` true)))
    (:`NewEnumerator1`
      (if _engagedinrun
        (setmembers `/Game/BPs/Data/Structs/F_PortalSystemData` :`StructRef` _portalsystemdata :`ReadyForInteractTrigger` true :`CurrentZoneActor` ZoneActorRef)))
    (:`NewEnumerator2`
      (if (not _engagedinrun)
        (setmembers `/Game/BPs/Data/Structs/F_PortalSystemData` :`StructRef` _portalsystemdata :`ReadyAtEntry` true :`DimensionPortal` ZoneActorRef)))
    (:`NewEnumerator4`
      (if _engagedinrun
        (message `/Game/BPs/Interfaces/BI_HyperMove.PassedZone` ZoneActorRef)))))

(event `/Game/BPs/Interfaces/BI_HyperMove.LeftZone`
  (params (ZoneType :type "/Game/BPs/Data/Enums/E_HyperZoneType Enum" :default "NewEnumerator0") (ZoneActorRef :type "Actor Object Reference"))
  (bind _portalsystemdata (`self.PortalSystemData`))
  (bind (_readyatentry _engagedinrun _dimensionportal) (break `/Game/BPs/Data/Structs/F_PortalSystemData` _portalsystemdata))
  (switch `/Game/BPs/Data/Enums/E_HyperZoneType` ZoneType
    (:`NewEnumerator0`
      (if _engagedinrun
        (setmembers `/Game/BPs/Data/Structs/F_PortalSystemData` :`StructRef` _portalsystemdata :`ReadyForSuperShift` false)))
    (:`NewEnumerator1`
      (if _engagedinrun
        (setmembers `/Game/BPs/Data/Structs/F_PortalSystemData` :`StructRef` _portalsystemdata :`ReadyForInteractTrigger` false :`CurrentZoneActor` null)))
    (:`NewEnumerator2`
      (if (not _engagedinrun)
        (setmembers `/Game/BPs/Data/Structs/F_PortalSystemData` :`StructRef` _portalsystemdata :`ReadyAtEntry` false :`DimensionPortal` null)))))

(event `EngagePortalRun`
  (message `/Game/BPs/Interfaces/BI_HyperMove.PortalRunEngaged` (`.DimensionPortal_5_C35091C449692A4F8B4C5A89241C304F` (break `/Game/BPs/Data/Structs/F_PortalSystemData` (`self.PortalSystemData`)))))

(event `/Game/BPs/Interfaces/BI_HyperMove.TriggerHyperMoveInteractionAction`
  (params (HyperMoveType :type "/Game/BPs/Data/Enums/E_HyperMoveInteractType Enum" :default "NewEnumerator3") (metadata :type "/Game/BPs/Data/Structs/F_HyperMoveInteractionActionData Structure") (Caller :type "Actor Object Reference"))
  (bind (_direction _force) (break `/Game/BPs/Data/Structs/F_HyperMoveInteractionActionData` metadata))
  (switch `/Game/BPs/Data/Enums/E_HyperMoveInteractType` HyperMoveType
    (:`NewEnumerator0`
      ; add world offset so GroundCheck does not override, reset grounded state so inertia isnt calculated by ground directional vecotrs, apply inertial vector
      (`SceneComponent.K2_AddWorldOffset` (`self.Capsule`) (0.0 0.0 10.0) false true)
      (set `self.bGrounded` false)
      (set `self.ComposedInertia` (+ (* (`KismetMathLibrary.GreaterGreater_VectorRotator` (* _direction _force) (`SceneComponent.K2_GetComponentRotation` (`self.Capsule`))) 0.25) (`self.ComposedInertia`)))
      ;; TODO: reproject innertia when bouncing
      (setmembers `/Game/BPs/Data/Structs/F_AxisInertia` :`StructRef` (`self.FrontAxis_S`) :`CurrentSpeed` 0.0)
      (setmembers `/Game/BPs/Data/Structs/F_AxisInertia` :`StructRef` (`self.SideAxis_S`) :`CurrentSpeed` 0.0))))

(fn `AccelerateAxis`
  (params (Axis :type "/Game/BPs/Data/Structs/F_AxisInertia Structure (by ref)") (IAValue :type "Float (double-precision)"))
  (bind (_axis _currentspeed _isbeingchanged _accel _decel _bypassdecel _maxpositive _maxnegative) (break `/Game/BPs/Data/Structs/F_AxisInertia` Axis))
  (if (!= IAValue 0.0)
    (setmembers `/Game/BPs/Data/Structs/F_AxisInertia` :`StructRef` Axis :`CurrentSpeed` (`KismetMathLibrary.FClamp` (+ _currentspeed (* _accel (`self.DT`) IAValue)) _maxnegative _maxpositive) :`IsBeingChanged` true)
    (else
      (setmembers `/Game/BPs/Data/Structs/F_AxisInertia` :`StructRef` Axis :`IsBeingChanged` false))))

(fn `DecelerateAxis`
  (params (DT :type "Float (double-precision)") (AxisRef :type "/Game/BPs/Data/Structs/F_AxisInertia Structure (by ref)"))
  (bind (_axis _currentspeed _isbeingchanged _accel _decel _bypassdecel) (break `/Game/BPs/Data/Structs/F_AxisInertia` AxisRef))
  (bind _returnvalue (* _decel DT))
  (if (`KismetMathLibrary.BooleanNOR` _isbeingchanged _bypassdecel)
    (if (and (> _currentspeed -20.0) (< _currentspeed 20.0))
      (setmembers `/Game/BPs/Data/Structs/F_AxisInertia` :`StructRef` AxisRef :`CurrentSpeed` 0.0)
      (else
        (setmembers `/Game/BPs/Data/Structs/F_AxisInertia` :`StructRef` AxisRef :`CurrentSpeed` (+ _currentspeed (`KismetMathLibrary.SelectFloat` _returnvalue (* _returnvalue -1.0) (> _currentspeed 0.0))))))
    (return)))

(fn `GetMultiGroundDirectionalVector`
  (returns (ForwardHit :type Boolean) (ForwardDirection :type "Vector Structure") (SideHit :type Boolean) (SideDirection :type "Vector Structure"))
  (bind _capsule (`self.Capsule`))
  (bind _capsule_2 (`self.Capsule`))
  (bind _returnvalue (`SceneComponent.GetForwardVector` _capsule_2))
  (bind _returnvalue_2 (`SceneComponent.K2_GetComponentLocation` (`self.Capsule`)))
  (bind _returnvalue_3 (`SceneComponent.K2_GetComponentLocation` (`self.Capsule`)))
  (bind _returnvalue_4 (`SceneComponent.K2_GetComponentLocation` (`self.Capsule`)))
  (bind _returnvalue_5 (`SceneComponent.GetRightVector` _capsule))
  (bind _returnvalue_6 (`SceneComponent.K2_GetComponentLocation` (`self.Capsule`)))
  (bind _returnvalue_7 (`KismetMathLibrary.NegateVector` (`SceneComponent.GetUpVector` _capsule)))
  (bind _returnvalue_8 (`KismetMathLibrary.NegateVector` (`SceneComponent.GetUpVector` _capsule_2)))
  (`|ExecutionSequence`
    (:`then_0`
      (bind (_outhit _returnvalue_9) (`KismetSystemLibrary.LineTraceSingle` :`Start` _returnvalue_4 :`End` (+ (+ (* _returnvalue -20.0) (* _returnvalue_8 120.0)) _returnvalue_4) :`TraceChannel` "TraceTypeQuery1" :`DrawDebugType` "ForOneFrame"))
      (bind (_outhit_2 _returnvalue_10) (`KismetSystemLibrary.LineTraceSingle` :`Start` _returnvalue_3 :`End` (+ (+ (* _returnvalue 20.0) (* _returnvalue_8 120.0)) _returnvalue_3) :`TraceChannel` "TraceTypeQuery1" :`DrawDebugType` "ForOneFrame"))
      (bind (_outhit_3 _returnvalue_11) (`KismetSystemLibrary.LineTraceSingle` :`Start` _returnvalue_6 :`End` (+ (+ (* _returnvalue_5 -20.0) (* _returnvalue_7 120.0)) _returnvalue_6) :`TraceChannel` "TraceTypeQuery1" :`DrawDebugType` "ForOneFrame"))
      (bind (_outhit_4 _returnvalue_12) (`KismetSystemLibrary.LineTraceSingle` :`Start` _returnvalue_2 :`End` (+ (+ (* _returnvalue_5 20.0) (* _returnvalue_7 120.0)) _returnvalue_2) :`TraceChannel` "TraceTypeQuery1" :`DrawDebugType` "ForOneFrame"))
      (return (and _returnvalue_9 _returnvalue_10) (`KismetMathLibrary.Normal` (- (`.Location` (`GameplayStatics.BreakHitResult` _outhit_2)) (`.Location` (`GameplayStatics.BreakHitResult` _outhit)))) (and _returnvalue_11 _returnvalue_12) (`KismetMathLibrary.Normal` (- (`.Location` (`GameplayStatics.BreakHitResult` _outhit_4)) (`.Location` (`GameplayStatics.BreakHitResult` _outhit_3))))))))

(fn `GroundCheckOffset`
  (returns (ReturnValue :type Boolean))
  (bind _capsule (`self.Capsule`))
  (bind _returnvalue (`SceneComponent.K2_GetComponentLocation` _capsule))
  (bind _capsulehalfheight (`CapsuleComponent.CapsuleHalfHeight` _capsule))
  (bind (_outhit _returnvalue_2) (`KismetSystemLibrary.LineTraceSingle` :`Start` _returnvalue :`End` (+ _returnvalue (* (`SceneComponent.GetUpVector` _capsule) _capsulehalfheight -1.02)) :`TraceChannel` "TraceTypeQuery1" :`DrawDebugType` "ForOneFrame" :`TraceColor` (struct :`R` 1.0 :`B` 0.762481 :`A` 1.0) :`TraceHitColor` (struct :`R` 1.0 :`G` 0.891841 :`A` 1.0)))
  (`|ExecutionSequence`
    (:`then_0`
      (if _returnvalue_2
        (`SceneComponent.K2_SetWorldLocation` (`self.Capsule`) (+ (`.Location` (`GameplayStatics.BreakHitResult` _outhit)) (`KismetMathLibrary.MakeVector` 0.0 0.0 _capsulehalfheight)) false true)))
    (:`then_1`
      (return _returnvalue_2))))

(fn `SwapMovementMode`
  (params (HyperMode :type Boolean))
  (bind _frontaxis_s (`self.FrontAxis_S`))
  (bind _portalsystemdata (`self.PortalSystemData`))
  (bind _frontaxis_hyper (`self.FrontAxis_Hyper`))
  (bind _returnvalue (pcsubsystem `EnhancedInputLocalPlayerSubsystem` (`GameplayStatics.GetPlayerController` 0)))
  (`|ExecutionSequence`
    (:`then_0`
      (setmembers `/Game/BPs/Data/Structs/F_HyperMoveData` :`StructRef` (`self.HyperMoveData`) :`bHyperMode` HyperMode)
      (`EnhancedInputSubsystemInterface.AddMappingContext` _returnvalue (select `bool` HyperMode :`false` "/Game/Core/Input/Standard/IMC_Standard.IMC_Standard" :`true` "/Game/Core/Input/Hyper/IMC_Hyper.IMC_Hyper" :!type "InputMappingContext Object Reference") 0 (struct))
      (`EnhancedInputSubsystemInterface.RemoveMappingContext` _returnvalue (select `bool` HyperMode :`false` "/Game/Core/Input/Hyper/IMC_Hyper.IMC_Hyper" :`true` "/Game/Core/Input/Standard/IMC_Standard.IMC_Standard" :!type "InputMappingContext Object Reference") (struct)))
    (:`then_1`
      (if HyperMode
        (setmembers `/Game/BPs/Data/Structs/F_AxisInertia` :`StructRef` _frontaxis_hyper :`CurrentSpeed` (`.CurrentSpeed_48_BCC8F5724ACD309D8CD3E488248F36B0` (break `/Game/BPs/Data/Structs/F_AxisInertia` _frontaxis_s)))
        (setmembers `/Game/BPs/Data/Structs/F_HyperMoveData` :`StructRef` (`self.HyperMoveData`) :`YawMomentum` 0.0)
        (else
          (setmembers `/Game/BPs/Data/Structs/F_AxisInertia` :`StructRef` _frontaxis_s :`CurrentSpeed` (`.CurrentSpeed_48_BCC8F5724ACD309D8CD3E488248F36B0` (break `/Game/BPs/Data/Structs/F_AxisInertia` _frontaxis_hyper)))
          (message `/Game/BPs/Interfaces/BI_HyperMove.PortalRunDisengaged` (`.DimensionPortal_5_C35091C449692A4F8B4C5A89241C304F` (break `/Game/BPs/Data/Structs/F_PortalSystemData` _portalsystemdata)))
          (setmembers `/Game/BPs/Data/Structs/F_PortalSystemData` :`StructRef` _portalsystemdata :`EngagedInRun` false :`DimensionPortal` null :`ReadyForInteractTrigger` false :`ReadyForSuperShift` false)
          (setmembers `/Game/BPs/Data/Structs/F_AxisInertia` :`StructRef` (`self.FrontAxis_Hyper`) :`IsBeingChanged` false))))))

(fn `UserConstructionScript`
  (bind _capsule (`self.Capsule`))
  (`SceneComponent.K2_AddLocalOffset` _capsule (`KismetMathLibrary.MakeVector` 0.0 0.0 (`CapsuleComponent.CapsuleHalfHeight` _capsule)) true true))