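; Experimental physics shard actor that currently only debug-draws a ray direction field built by geodesic-style triangle subdivision.
; Each tick, FoldSphere subdivides one tetrahedral face twice with normalization, and Iteration2 draws the vertices and centers as rays.
; A disconnected solver ray-casts a sphere of directions, wakes hit actors, turns compression into curve-driven push-back and damping, flips momentum past the limit, then moves the actor.
; Construction sizes the debug and radius spheres.
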(event Custom|DBGPost
  ;[0.15 0.15 0.15 0.5] DBG Post
  (Utilities|DebugM
    (:True
      (Development|PrintText (Utilities|Text|FormatText "HitCount {hc} 
DiffSumLength: {dsl}" (stale _hitcount)) true true "(R=1.000000,G=0.161997,B=0.646574,A=1.000000)" 2.0 "PhysShard")
      (CallFunction|DebugRayLocalwithOffset (stale _hitdiffsum) 1e+02 0.0 "0, 0, 0" "(R=0.354447,G=1.000000,B=0.891047,A=1.000000)")
      (CallFunction|DebugRayLocalwithOffset (Variables|Default|GetMomentumVector) 1e+02 0.0 "0, 0, 0" "(R=1.000000,G=0.422321,B=0.218750,A=1.000000)"))))

(event EventBeginPlay)

(event Collision|EventActorBeginOverlap
  (params (OtherActor :type Actor%20Object%20Reference)))

(event EventTick
  (params (DeltaSeconds :type Float%20%28single-precision%29))
  (Utilities|FlowControl|Sequence
    (:then_2
      (CallFunction|Iteration2))))

(event EventTriggerWakeUp
  ;[0.15 0.15 0.15 0.5] Stopped
  ;;[0.15 0.15 0.15 0.5] WakeUp
)

(event Custom|Iteration2
  (bind _vectrigs (CallFunction|FoldSphere 2))
  (for _array_element _vectrigs
    (CallFunction|DebugRayLocalwithOffset (.com _array_element) (Variables|Default|GetRadius) 0.0 "0, 0, 0" "(R=1.000000,G=1.000000,B=0.000000,A=1.000000)")
    (for _array_element_2 (Utilities|Array|MakeArray (.v1 _array_element) (.v2 _array_element) (.v3 _array_element))
      (CallFunction|DebugRayLocalwithOffset _array_element_2 (Variables|Default|GetRadius) 0.0 "0, 0, 0" "(R=1.000000,G=1.000000,B=1.000000,A=1.000000)"))))

(fn ConstructionScript
  (bind _radius (Variables|Default|GetRadius))
  (Transformation|SetRelativeScale3D (Variables|Default|GetDBG) (Math|Conversions|ToVector(Float) (/ _radius 5e+01)))
  (Components|Sphere|SetSphereRadius (Variables|Default|GetSphere1) (* _radius (Variables|Default|GetCompressionDistanceNormal)) false)
  (Components|Sphere|SetSphereRadius (Variables|Default|GetRadii) _radius false))

(fn FieldRayCast
  (params (FieldVectors :type Array%20of%20Vectors))
  (bind _hitnorms (LocalVariables|GetHitNorms))
  (bind _defaultsceneroot (Variables|Default|GetDefaultSceneRoot))
  (bind _returnvalue (Transformation|GetAttachParent _defaultsceneroot))
  (Utilities|FlowControl|Sequence
    (:then_0
      (Utilities|Array|Clear (LocalVariables|GetHitNorms))
      (LocalVariables|SetHitDiffSumI "0, 0, 0")
      (Utilities|Array|Clear (LocalVariables|GetHitDifsArr)))
    (:then_1
      (for _array_element FieldVectors
        (bind (_hitresult _bhit) (CallFunction|RayCast "0, 0, 0" _array_element (* (Variables|Default|GetRadius) 1.05) (Math|Float|SelectFloat 0.0 -1.0 (Variables|Default|GetDebug)) (select (Utilities|IsValid _returnvalue) _returnvalue _defaultsceneroot) true "(R=1.000000,G=1.000000,B=1.000000,A=1.000000)" "(R=0.000000,G=1.000000,B=1.000000,A=1.000000)"))
        (if _bhit
          (Class|BIPhysicsShard|TriggerWakeUp(Message) (.HitActor (Collision|BreakHitResult _hitresult)))
          (Utilities|Array|Add (LocalVariables|GetHitNorms) (.ImpactNormal (Collision|BreakHitResult _hitresult)))
          (bind _output_get (LocalVariables|SetHitDiffSumI (+ (stale _output_get) (- (.ImpactPoint (Collision|BreakHitResult _hitresult)) (.TraceEnd (Collision|BreakHitResult _hitresult))))))
          (Utilities|Array|Add (LocalVariables|GetHitDifsArr) (- (.ImpactPoint (Collision|BreakHitResult _hitresult)) (.TraceEnd (Collision|BreakHitResult _hitresult)))))))
    (:then_2
      (return _hitnorms (LocalVariables|GetHitDifsArr) (LocalVariables|GetHitDiffSumI) (> (Math|Vector|VectorLength (LocalVariables|GetHitDiffSumI)) 0.0) (Utilities|Array|Length _hitnorms)))))

(fn CalculateReDirectionVector
  (params (Normals :type Array%20of%20Vectors))
  (LocalVariables|SetSum "0, 0, 0")
  (for _array_element Normals
    (bind _output_get (LocalVariables|SetSum (+ (stale _output_get) _array_element))))
  (bind _output_get_2 (LocalVariables|SetSum (/ (stale _output_get_2) (Utilities|Array|Length Normals))))
  (return (Math|Vector|Normalize (/ _output_get_2 (Utilities|Array|Length Normals)))))

(fn DebugRayLocalwithOffset
  (params (Direction :type Vector) (Distance :type Float%20%28double-precision%29) (Duration :type Float%20%28double-precision%29) (Offset :type Vector) (TraceColor :type Linear%20Color%20Structure) (TraceHit :type Linear%20Color%20Structure))
  (CallFunction|RayCast (+ (Transformation|GetWorldLocation (Variables|Default|GetDefaultSceneRoot)) Offset) Direction Distance Duration 0 false TraceColor TraceHit)
  (return))

(fn GetLongestVector
  (params (HitDiffs :type Array%20of%20Vectors))
  (LocalVariables|SetIdx 0)
  (LocalVariables|SetLargest "0, 0, 0")
  (for (_array_element _array_index) HitDiffs
    (if (> (Math|Vector|VectorLength _array_element) (Math|Vector|VectorLength (LocalVariables|GetLargest)))
      (LocalVariables|SetLargest _array_element)
      (LocalVariables|SetIdx _array_index)))
  (return (LocalVariables|GetLargest) (LocalVariables|GetIdx)))

(fn SphereVectorArray
  (params (RaysPerCircle :type Integer) (AttachToParent :type Boolean) (Parent :type Scene%20Component%20Object%20Reference))
  (bind _returnvalue (Math|Float|MakeLiteralFloat 1.8e+02))
  (bind _returnvalue_2 (Math|Integer|%(Integer) RaysPerCircle 2))
  (bind _returnvalue_3 (+ RaysPerCircle _returnvalue_2))
  (bind _returnvalue_4 (/ _returnvalue_3 2))
  (bind _returnvalue_5 (Math|Conversions|ToFloat(Integer) _returnvalue_4))
  (bind _returnvalue_6 (/ _returnvalue _returnvalue_5))
  (Utilities|FlowControl|Sequence
    (:then_0
      (Utilities|Array|Clear (LocalVariables|GetHalph2DCircle))
      (Utilities|Array|Clear (LocalVariables|GetFullSphere))
      (Utilities|Array|Clear (LocalVariables|GetLocalAxes)))
    (:then_1
      (if AttachToParent
        ;[0.15 0.15 0.15 0.5] Object local axes config
        (Utilities|IsValid Parent
          (:Is%20Valid
            (LocalVariables|SetLocalAxes (Utilities|Array|MakeArray (Math|Vector|GetForwardVector Parent) (Math|Vector|GetRightVector Parent) (Math|Vector|GetUpVector Parent))))
          (:Is%20Not%20Valid
            (Development|PrintString "Null Parent in sphere ray array creation" true true "(R=0.197917,G=0.000000,B=0.000000,A=1.000000)" 2.0 "ShardSphere")))
        (else
          ;[0.15 0.15 0.15 0.5] Global axes
          (LocalVariables|SetLocalAxes (Utilities|Array|MakeArray "1.000000,0.000000,0.000000" "0.000000,1.000000,0.000000" "0.000000,0.000000,1.000000")))))
    (:then_2
      ;[0.15 0.15 0.15 0.5] Half cirlcle without edge vectors around Z
      (for _index (range 0 (- _returnvalue_4 1))
        (Utilities|Array|Add (LocalVariables|GetHalph2DCircle) (Math|Vector|RotateVectorAroundAxis (Utilities|Array|Get(acopy) (LocalVariables|GetLocalAxes)) (* _index _returnvalue_6) (Utilities|Array|Get(acopy) (LocalVariables|GetLocalAxes) 2)))))
    (:then_3
      ;[0.15 0.15 0.15 0.5] Full circle encapsulation
      (for _array_element (LocalVariables|GetHalph2DCircle)
        (for _index_2 (range 0 (* _returnvalue_4 2))
          (Utilities|Array|Add (LocalVariables|GetFullSphere) (Math|Vector|RotateVectorAroundAxis _array_element (* _index_2 _returnvalue_6) (Utilities|Array|Get(acopy) (LocalVariables|GetLocalAxes)))))))
    (:then_5
      (return (LocalVariables|GetFullSphere)))))

(fn DotNormalizedVectorfromHitDiffs
  (params (HitDiffs :type Array%20of%20Vectors) (HitDiffSum :type Vector) (Momentum :type Vector))
  (bind _returnvalue (Math|Vector|Normalize HitDiffSum))
  (LocalVariables|SetDotNormalized "0, 0, 0")
  (for _array_element HitDiffs
    (bind _output_get (LocalVariables|SetDotNormalized (+ (stale _output_get) (* _returnvalue (* (Math|Vector|VectorLength _array_element) (Math|Vector|DotProduct (Math|Vector|Normalize _array_element) (Math|Vector|NegateVector _returnvalue))))))))
  (bind _output_get_2 (LocalVariables|SetDotNormalized (/ (stale _output_get_2) (Utilities|Array|Length HitDiffs))))
  (return _output_get_2))

(fn MovingAverage
  (params (Count :type Integer) (Value :type Float%20%28double-precision%29) (ArrayToSave :type Array%20of%20Floats%20%28double-precision%29))
  (bind _returnvalue (Utilities|Array|Length ArrayToSave))
  (if (< _returnvalue Count)
    (Utilities|Array|SetArrayElem ArrayToSave (+ _returnvalue 1) Value true)
    (LocalVariables|SetAve 0.0 :!label _label)
    (for _array_element ArrayToSave
      (bind _output_get (LocalVariables|SetAve (+ (stale _output_get) _array_element))))
    (return (/ _output_get Count))
    (else
      (for _index (range 1 (- Count 1))
        (Utilities|Array|SetArrayElem ArrayToSave _index (Utilities|Array|Get(acopy) ArrayToSave (- _index 1))))
      (Utilities|FlowControl|Sequence
        (:then_0
          (Utilities|Array|SetArrayElem ArrayToSave (- Count 1) Value))
        (:then_1
          (goto _label))))))

(fn ComandDiffsComDifference
  (params (Diffs :type Array%20of%20Vectors))
  (for _array_element Diffs
    (bind _output_get (LocalVariables|SetSum (+ (stale _output_get) (Math|Vector|Normalize _array_element)))))
  (bind _output_get_2 (LocalVariables|SetSum (/ (stale _output_get_2) (Utilities|Array|Length Diffs))))
  (return (- (LocalVariables|GetSum) (Math|Vector|VectorZero)) (Math|Vector|VectorLength (LocalVariables|GetSum))))

(fn FoldSphere
  (params (SubDivisions :type Integer))
  (bind _returnvalue (Class|KismetMathLibrary|VectorRight))
  (bind _returnvalue_2 (Class|KismetMathLibrary|VectorForward))
  (bind _returnvalue_3 (Math|Vector|VectorUp))
  (bind _trigspheredoublerot (LocalVariables|GetTrigSphereDoubleRot))
  (bind _returnvalue_4 (Math|Vector|RotateVectorAroundAxis _returnvalue -3e+01 _returnvalue_2))
  (Utilities|FlowControl|Sequence
    (:then_0
      (Utilities|Array|Clear (LocalVariables|GetTrigSphereBase))
      (Utilities|Array|Clear (LocalVariables|GetTrigSphereFull)))
    (:then_1
      (bind _vectrig (CallFunction|VectorTrigForm _returnvalue_3 (Math|Vector|RotateVectorAroundAxis _returnvalue_4 1.2e+02 _returnvalue_3) (Math|Vector|RotateVectorAroundAxis _returnvalue_4 -1.2e+02 _returnvalue_3)))
      (bind _copy (CallFunction|CalculateTrigCrossCenter _vectrig))
      (LocalVariables|SetTrigSphereFull (Utilities|Array|MakeArray _copy))
      ;[0.15 0.15 0.15 0.5] Subdivide, clear, set, repeat
      (for _index (range 0 (- SubDivisions 1))
        (bind _subdivisions (CallFunction|SubdivideTrigs (LocalVariables|GetTrigSphereFull) true))
        (LocalVariables|SetTrigSphereFull _subdivisions))
      (for (_ _array_index) _trigspheredoublerot
        (CallFunction|RotateTrigAroundAxis (Utilities|Array|Get(acopy) _trigspheredoublerot _array_index) "1.000000,0.000000,0.000000" (Variables|Default|GetDBG1))
        (CallFunction|RotateTrigAroundAxis (Utilities|Array|Get(acopy) _trigspheredoublerot _array_index) "0.000000,1.000000,0.000000" (Variables|Default|GetDBG2))
        (CallFunction|RotateTrigAroundAxis (Utilities|Array|Get(acopy) _trigspheredoublerot _array_index) "0.000000,0.000000,1.000000" (Variables|Default|GetDBG3)))
      (Utilities|FlowControl|Sequence
        (:then_0
          (for _array_element (LocalVariables|GetTrigSphereFull)
            (CallFunction|DebugRayLocalwithOffset (.com _array_element) (Variables|Default|GetRadius) 0.0 "0, 0, 0" "(R=1.000000,G=0.000000,B=0.000000,A=1.000000)"))
          (for _array_element_2 (LocalVariables|GetTrigSphereDoubleRot)
            (CallFunction|DebugRayLocalwithOffset (.com _array_element_2) (Variables|Default|GetRadius) 0.0 "0, 0, 0" "(R=1.000000,G=0.876426,B=0.000000,A=1.000000)")))
        (:then_1
          (return (LocalVariables|GetTrigSphereFull)))))))